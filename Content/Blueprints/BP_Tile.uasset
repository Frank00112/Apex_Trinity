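; BP_Tile is a board tile actor that shows highlight states for movement, attack and unit selection.
; Movement, attack and selection events toggle a shared HighlightMesh and swap its material, with selection choosing a per-player material from TeamID.
; A separate event applies a border material to the tile's static mesh.
; It has no tick or startup logic, so other objects drive every visual change.
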(event EventBeginPlay)

(event Collision|EventActorBeginOverlap
  (params (OtherActor :type Actor%20Object%20Reference)))

(event EventTick
  (params (DeltaSeconds :type Float%20%28single-precision%29)))

(event EventSetMovementHighlight
  (params (bIsOn :type Boolean))
  (Rendering|SetVisibility (Variables|Default|GetHighlightMesh) bIsOn false)
  (Rendering|Material|SetMaterial (Variables|Default|GetHighlightMesh) 0 "/Game/Materials/M_Highlight_Move.M_Highlight_Move"))

(event EventSetAttackHighlight
  (params (bIsOn :type Boolean))
  (Rendering|SetVisibility (Variables|Default|GetHighlightMesh) bIsOn false)
  (Rendering|Material|SetMaterial (Variables|Default|GetHighlightMesh) 0 "/Game/Materials/M_Highlight_Attack.M_Highlight_Attack"))

(event EventSetSelectionHighlight
  (params (bIsOn :type Boolean) (TeamID :type Integer))
  (bind _highlightmesh (Variables|Default|GetHighlightMesh))
  (if bIsOn
    (Rendering|SetVisibility _highlightmesh true false)
    (Rendering|Material|SetMaterial _highlightmesh 0 (Utilities|Select :Index TeamID :Option%200 "/Game/Materials/M_Select_Player0.M_Select_Player0" :Option%201 "/Game/Materials/M_Select_Player1.M_Select_Player1"))
    (else
      (Rendering|SetVisibility (Variables|Default|GetHighlightMesh) false false))))

(event EventApplyBorderMaterial
  (Rendering|Material|SetMaterial (Variables|Default|GetStaticMeshComponent) 0 "/Game/Materials/M_Border.M_Border"))

(fn ConstructionScript)